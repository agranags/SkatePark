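; Spline-driven construction Blueprint that lays a chosen static mesh, with two material slots, along a spline as deformed spline mesh components.
; The construction script calls a Wire graph, where SplineMeshVar selects how the spline is segmented.
; The default mode builds one segment per point pair using point tangents.
; The alternative cuts the length into fixed Spacing steps, with tangents from spline direction scaled by Spacing plus TangentScaleAdd.
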(fn ConstructionScript
  (|Wire))